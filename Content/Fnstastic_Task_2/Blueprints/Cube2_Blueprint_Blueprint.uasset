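; Cube2_Blueprint is an interactable actor that spawns a BP_Fox AI pawn at one of three tagged spawn points.
; OnIntaraction switches on NumberOfFox to pick tag Spawn1, Spawn2 or Spawn3, then copies that number to the spawned fox.
; FindTagetByTag locates the spawn point by scanning every actor in the level and returning the first with the matching tag.
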(event EventOnIntaraction
  (switch int (Variables|Default|Getnumber%20of%20fox)
    (:0
      (bind _target (CallFunction|FindTagetbyTag "Spawn1"))
      (bind _returnvalue (AI|SpawnAIFromClass "/Game/Fnstastic_Task_2/Blueprints/BP_Fox.BP_Fox_C" 0 (Transformation|GetActorLocation _target) "0, 0, 0" false 0))
      (bind _asbp_fox (Utilities|Casting|CastToBP_Fox _returnvalue))
      (Variables|/Game/Fnstastic_Task_2/Blueprints/BP_Fox.BP_Fox_C|SetNumber%20of%20Fox _asbp_fox (Variables|Default|Getnumber%20of%20fox)))
    (:1
      (bind _target_2 (CallFunction|FindTagetbyTag "Spawn2"))
      (bind _returnvalue_2 (AI|SpawnAIFromClass "/Game/Fnstastic_Task_2/Blueprints/BP_Fox.BP_Fox_C" 0 (Transformation|GetActorLocation _target_2) "0, 0, 0" false 0))
      (bind _asbp_fox_2 (Utilities|Casting|CastToBP_Fox _returnvalue_2))
      (Variables|/Game/Fnstastic_Task_2/Blueprints/BP_Fox.BP_Fox_C|SetNumber%20of%20Fox _asbp_fox_2 (Variables|Default|Getnumber%20of%20fox)))
    (:2
      (bind _target_3 (CallFunction|FindTagetbyTag "Spawn3"))
      (bind _returnvalue_3 (AI|SpawnAIFromClass "/Game/Fnstastic_Task_2/Blueprints/BP_Fox.BP_Fox_C" 0 (Transformation|GetActorLocation _target_3) "0, 0, 0" false 0))
      (bind _asbp_fox_3 (Utilities|Casting|CastToBP_Fox _returnvalue_3))
      (Variables|/Game/Fnstastic_Task_2/Blueprints/BP_Fox.BP_Fox_C|SetNumber%20of%20Fox _asbp_fox_3 (Variables|Default|Getnumber%20of%20fox)))))

(fn ConstructionScript
  (|CallParentFunction))

(fn FindTagetbyTag
  (params (Tag :type Name))
  (bind _outactors (Actor|GetAllActorsOfClass "/Script/Engine.Actor"))
  (bind _array_element (Utilities|Array|ForEachLoopwithBreak _outactors :!label _label)
    (:LoopBody
      (if (Actor|ActorHasTag _array_element Tag)
        (LocalVariables|SetL_Target _array_element)
        (goto _label Break)))
    (:Completed
      (return (LocalVariables|GetL_Target)))))