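; AI controller that drives a BP_Fox pawn with one of three movement patterns, selected by the fox's NumberOfFox.
; After a short BeginPlay delay workaround, it caches the pawn and finds finish actors by searching all actors for tags.
; Tick runs DoOnce-gated AIMoveTo loops reset by delays: move to the finish, stop-and-go toward it, or alternate on timers between forward and reverse targets.
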(event EventBeginPlay
  ;[0 0 0] Fix bug
  (Utilities|FlowControl|Delay 0.2)
  (bind _output_get (Variables|Default|SetFox_Ref (.AsBP%20Fox (Utilities|Casting|CastToBP_Fox (Pawn|GetControlledPawn)))))
  (bind _output_get_2 (Variables|Default|SetNumber%20of%20Fox (Variables|/Game/Fnstastic_Task_2/Blueprints/BP_Fox.BP_Fox_C|GetNumber%20of%20Fox _output_get)))
  (switch int _output_get_2
    (:0
      (bind _target (CallFunction|FindTagetbyTag "Finish1"))
      (Variables|Default|SetTarget _target))
    (:1
      (bind _target_2 (CallFunction|FindTagetbyTag "Finish2"))
      (Variables|Default|SetTarget _target_2))
    (:2
      (bind _target_3 (CallFunction|FindTagetbyTag "Finish3"))
      (Variables|Default|SetTarget _target_3)
      (bind _target_4 (CallFunction|FindTagetbyTag "Finish3Revers"))
      (Variables|Default|SetTargetRevers _target_4))))

(event EventTick
  (params (DeltaSeconds :type Float%20%28single-precision%29))
  (switch int (Variables|Default|GetNumber%20of%20Fox)
    (:0
      (Utilities|FlowControl|Delay 1.0)
      ;[1 1 1] движение 1
      (Utilities|FlowControl|DoOnce false :!label _label
        (:Completed
          (AI|AIMoveTo (Variables|Default|GetFox_Ref) "0, 0, 0" (Variables|Default|GetTarget) 5.0 false
            (:OnSuccess
              _)
            (:OnFail
              _))
          (Utilities|FlowControl|Delay 1.0)
          (goto _label Reset))))
    (:1
      ;[1 1 1] движение 2
      (Utilities|FlowControl|DoOnce false :!label _label_2
        (:Completed
          (AI|AIMoveTo (Variables|Default|GetFox_Ref) "0, 0, 0" (Variables|Default|GetTarget) 5.0 false
            (:then
              (Utilities|FlowControl|Delay 1.0)
              (AI|Navigation|StopMovement)
              (Utilities|FlowControl|Delay 0.5)
              (goto _label_2 Reset))))))
    (:2
      ;[1 1 1] Движение 3
      (Utilities|FlowControl|DoOnce false :!label _label_3
        (:Completed
          (AI|AIMoveTo (Variables|Default|GetFox_Ref) "0, 0, 0" (Variables|Default|GetTarget) 5.0 false
            (:then
              (Utilities|FlowControl|Delay 1.0)
              (AI|AIMoveTo (Variables|Default|GetFox_Ref) "0, 0, 0" (Variables|Default|GetTargetRevers) 5.0 false
                (:then
                  _)
                (:OnSuccess
                  _)
                (:OnFail
                  _))
              (Utilities|FlowControl|Delay 0.5)
              (goto _label_3 Reset))))))))

(fn ConstructionScript)

(fn FindTagetbyTag
  (params (Tag :type Name))
  (bind _outactors (Actor|GetAllActorsOfClass "/Script/Engine.Actor"))
  (bind _array_element (Utilities|Array|ForEachLoopwithBreak _outactors :!label _label)
    (:LoopBody
      (if (Actor|ActorHasTag _array_element Tag)
        (LocalVariables|SetL_Target _array_element)
        (goto _label Break)))
    (:Completed
      (return (LocalVariables|GetL_Target)))))